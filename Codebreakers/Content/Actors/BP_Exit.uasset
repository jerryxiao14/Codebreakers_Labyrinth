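; BP_Exit is a level exit actor that shows the win menu when its mesh is overlapped.
; On BeginPlay it registers itself as ExitMesh on the GS_EasyLevel game state.
; A custom event switches the mesh to OverlapAllDynamic collision, with no caller in this graph.
; Any overlap, without filtering the other actor, creates W_WinMenu, sets UI-only input and shows the mouse cursor.
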(event OnComponentBeginOverlap(StaticMesh)
  (params (OverlappedComponent :type Primitive%20Component%20Object%20Reference) (OtherActor :type Actor%20Object%20Reference) (OtherComp :type Primitive%20Component%20Object%20Reference) (OtherBodyIndex :type Integer) (bFromSweep :type Boolean) (SweepResult :type Hit%20Result%20Structure%20%28by%20ref%29))
  (bind _returnvalue (Game|GetPlayerController 0))
  (Input|SetInputModeUIOnly _returnvalue 0 "DoNotLock" false)
  (Variables|/Script/Engine.PlayerController|SetbShowMouseCursor _returnvalue true)
  (bind _returnvalue_2 (UserInterface|CreateWidget "/Game/Widgets/Menus/W_WinMenu.W_WinMenu_C"))
  (UserInterface|Viewport|AddtoViewport _returnvalue_2 0))

(event Custom|Enable%20OverlapAllDynamic
  ;[0.15 0.15 0.15 0.5] Enable OverlapAllDynamic
  (Collision|SetCollisionProfileName (Variables|Default|GetStaticMesh) "OverlapAllDynamic" true :!class /Script/Engine.PrimitiveComponent))

(event EventBeginPlay
  (bind _asgs_easy_level (Utilities|Casting|CastToGS_EasyLevel (Game|GetGameState)))
  (Variables|/Game/GameState/GS_EasyLevel.GS_EasyLevel_C|SetExitMesh _asgs_easy_level self))

(fn ConstructionScript)