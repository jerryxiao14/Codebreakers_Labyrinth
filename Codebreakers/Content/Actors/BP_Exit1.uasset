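; BP_Exit1 is a parkour exit pickup that awards a key and sends the overlapping actor back to a stored return point.
; On BeginPlay its mesh switches to the OverlapAllDynamic collision profile.
; Any overlap destroys it, increments GS_EasyLevel's key count, applies GI_Game's ReturnTransform and unloads the ParkourMap streaming level named from CurrentParkour minus one.
; Exit-mesh registration and win-menu logic are disconnected and never run.
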(event OnComponentBeginOverlap(StaticMesh)
  (params (OverlappedComponent :type Primitive%20Component%20Object%20Reference) (OtherActor :type Actor%20Object%20Reference) (OtherComp :type Primitive%20Component%20Object%20Reference) (OtherBodyIndex :type Integer) (bFromSweep :type Boolean) (SweepResult :type Hit%20Result%20Structure%20%28by%20ref%29))
  (Actor|DestroyActor)
  (CallFunction|IncrementKeys)
  (bind _asgi_game (Utilities|Casting|CastToGI_Game (Game|GetGameInstance)))
  (Transformation|SetActorTransform OtherActor (Variables|/Game/GameState/GI_Game.GI_Game_C|GetReturnTransform _asgi_game))
  (bind _asgs_easy_level (Utilities|Casting|CastToGS_EasyLevel (Game|GetGameState)))
  (Game|UnloadStreamLevel(byName) (Utilities|String|StringToName (Utilities|String|Append "ParkourMap" (Utilities|String|ToString(Integer) (- (Variables|/Game/GameState/GS_EasyLevel.GS_EasyLevel_C|GetCurrentParkour _asgs_easy_level) 1)))) true))

(event Custom|Enable%20OverlapAllDynamic
  ;[0.15 0.15 0.15 0.5] Enable OverlapAllDynamic
  (Collision|SetCollisionProfileName (Variables|Default|GetStaticMesh) "OverlapAllDynamic" true :!class /Script/Engine.PrimitiveComponent))

(event Custom|IncrementKeys
  (bind _asgs_easy_level (Utilities|Casting|CastToGS_EasyLevel (Game|GetGameState)))
  (Default|IncrementKeysObtained _asgs_easy_level))

(event EventBeginPlay
  (CallFunction|EnableOverlapAllDynamic))

(fn ConstructionScript)