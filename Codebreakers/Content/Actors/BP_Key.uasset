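; BP_Key is a key actor that opens a puzzle when something overlaps its sphere.
; The overlap disables player movement, switches to UI-only input with a visible cursor, and calls DisplayRandomPuzzle, which always selects multiple choice.
; That event fills a BP_MultipleChoice widget with a random question from the GS_EasyLevel game state, then destroys the key.
; A Hill Cipher widget event also exists but is not called here.
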(event OnComponentBeginOverlap(Sphere)
  (params (OverlappedComponent :type Primitive%20Component%20Object%20Reference) (OtherActor :type Actor%20Object%20Reference) (OtherComp :type Primitive%20Component%20Object%20Reference) (OtherBodyIndex :type Integer) (bFromSweep :type Boolean) (SweepResult :type Hit%20Result%20Structure%20%28by%20ref%29))
  (bind _returnvalue (Game|GetPlayerController 0))
  ;[0.15 0.15 0.15 0.5] Display Puzzle On Collison
  (Pawn|Components|CharacterMovement|DisableMovement (Variables|/Script/Engine.Character|GetCharacterMovement (Game|GetPlayerCharacter 0)))
  (Input|SetInputModeUIOnly _returnvalue 0 "DoNotLock" false)
  (Variables|/Script/Engine.PlayerController|SetbShowMouseCursor _returnvalue true)
  (CallFunction|DisplayRandomPuzzle))

(event Custom|Display%20Random%20Puzzle
  ;[0.15 0.15 0.15 0.5] Display Random Puzzle
  (CallFunction|DisplayMultipleChoicePuzzle))

(event Custom|Display%20Multiple%20Choice%20Puzzle
  ;[0.15 0.15 0.15 0.5] Display Multiple Choice Puzzle
  (bind _asgs_easy_level (Utilities|Casting|CastToGS_EasyLevel (Game|GetGameState)))
  (bind _question (Default|GetRandomQuestion _asgs_easy_level))
  (bind _returnvalue (UserInterface|CreateWidget "/Game/Widgets/BP_MultipleChoice.BP_MultipleChoice_C" 0 (.Question (Utilities|Struct|BreakST_Question _question)) (.ChoiceA (Utilities|Struct|BreakST_Question _question)) (.ChoiceB (Utilities|Struct|BreakST_Question _question)) (.ChoiceC (Utilities|Struct|BreakST_Question _question)) (.ChoiceD (Utilities|Struct|BreakST_Question _question)) (.CorrectAnswer (Utilities|Struct|BreakST_Question _question))))
  (UserInterface|Viewport|AddtoViewport _returnvalue 0)
  (Actor|DestroyActor))

(event Custom|Display%20Hill%20Cipher%20Widget
  ;[0.15 0.15 0.15 0.5] Display Hill Cipher Widget
  (bind _returnvalue (UserInterface|CreateWidget "/Game/Widgets/BP_HillCipher.BP_HillCipher_C"))
  (UserInterface|Viewport|AddtoViewport _returnvalue 0)
  (Actor|DestroyActor))

(fn ConstructionScript)